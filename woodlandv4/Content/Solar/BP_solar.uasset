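; BP_solar is a configurable celestial body that orbits a parent planet in a solar system scene.
; Its construction script snaps it to the ParentPlanet's sphere while keeping world rotation and scale.
; A spring arm sets the distance to the parent, the sphere takes the planet scale, and a RotatingMovement component supplies the rotation rate.
; All setup happens at construction, and the event graph has no active logic.
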(fn `UserConstructionScript`
  (`self.K2_AttachToComponent` (`/Game/Solar/BP_solar.Sphere` (`self.ParentPlanet`)) "None" "SnapToTarget" "KeepWorld" "KeepWorld")
  (set `SpringArmComponent.TargetArmLength` (`self.DistanceToParent`) (`self.SpringArm`))
  (`SceneComponent.SetWorldScale3D` (`self.Sphere`) (`self.PlanetScale`))
  (set `RotatingMovementComponent.RotationRate` (`self.RotationRate`) (`self.RotatingMovement`)))