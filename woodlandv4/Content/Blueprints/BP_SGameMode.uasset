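; BP_SGameMode is the game mode for a multiplayer BP_JellyPlane game, handling spawning, respawns, kill credit and the alive count.
; PostLogin has each player controller create its HUD, and ChoosePlayerStart hands out PlayerStarts by tagging each as "Taken".
; Respawn sends the controller to the first TriggerBox with no overlapping plane.
; ActorDead credits the killer, then recounts planes into PlayerAlive and pushes the count to their HUDs.
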(event `self.K2_PostLogin`
  (params (NewPlayer :type "PlayerController Object Reference"))
  (bind _asbp_player_controller (cast `/Game/Blueprints/BP_PlayerController` NewPlayer))
  (`/Game/Blueprints/BP_PlayerController.Client_CreateHUD` _asbp_player_controller))

(event `Respawn`
  (params (Controller :type "/Game/Blueprints/BP_PlayerController Object Reference"))
  (bind _outactors (`GameplayStatics.GetAllActorsOfClass` "/Script/Engine.TriggerBox"))
  (for _array_element _outactors
    (if (== (`KismetArrayLibrary.Array_Length` (`self.GetOverlappingActors` _array_element "/Game/Blueprints/JellyPlane/BP_JellyPlane.BP_JellyPlane_C")) 0)
      (`/Game/Blueprints/BP_PlayerController.Server_ReSpwan` Controller (`self.GetTransform` _array_element))
      (break))))

(event `ActorDead`
  (params (Player :type "/Game/Blueprints/JellyPlane/BP_JellyPlane Object Reference") (DeathCausor :type "/Game/Blueprints/JellyPlane/BP_JellyPlane Object Reference"))
  (bind _asbp_player_controller (cast `/Game/Blueprints/BP_PlayerController` (`Pawn.GetController` DeathCausor)))
  (`/Game/Blueprints/BP_PlayerController.IncreaseKiils` _asbp_player_controller)
  (bind _outactors (`GameplayStatics.GetAllActorsOfClass` "/Game/Blueprints/JellyPlane/BP_JellyPlane.BP_JellyPlane_C"))
  (for _array_element _outactors
    (bind _asbp_player_controller_2 (cast `/Game/Blueprints/BP_PlayerController` (`Pawn.GetController` _array_element)))
    (bind _returnvalue (`KismetArrayLibrary.Array_Length` _outactors))
    (`/Game/Blueprints/BP_PlayerController.ChangePlayerHUDStatus` _asbp_player_controller_2 _returnvalue)
    (set `self.PlayerAlive` _returnvalue)))

(event `self.ReceiveBeginPlay`
  (bind _outactors (`GameplayStatics.GetAllActorsOfClass` "/Game/Blueprints/JellyPlane/BP_JellyPlane.BP_JellyPlane_C"))
  (set `self.PlayerAlive` (`KismetArrayLibrary.Array_Length` _outactors)))

(fn `ChoosePlayerStart`
  (params (Player :type "Controller Object Reference"))
  (returns (ReturnValue :type "Actor Object Reference"))
  (bind _outactors (`GameplayStatics.GetAllActorsOfClass` "/Script/Engine.PlayerStart"))
  (bind _output_get (set `self.Spawning_Locations` _outactors))
  (for _array_element _output_get
    (if (!= (`PlayerStart.PlayerStartTag` _array_element) "Taken")
      (set `PlayerStart.PlayerStartTag` "Taken" _array_element)
      (return _array_element))))

(fn `UserConstructionScript`)